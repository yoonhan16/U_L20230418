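; BP_P-38 is a P-38 aircraft pawn that flies forward automatically.
; Each tick it adds full movement input along its forward vector and spins the left and right propellers.
; PropRotate rolls the given propeller by a speed variable scaled by delta time.
; The IA_Pitch Enhanced Input action only prints its value and does not yet affect flight.
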(event `self.ReceiveTick`
  (params (DeltaSeconds :type "Float (single-precision)"))
  (`|ExecutionSequence`
    (:`then_0`
      (`self.AddMovementInput` (`self.GetActorForwardVector`)))
    (:`then_1`
      (`self.Prop_Rotate` (`self.P-38 Left Prop`)))
    (:`then_2`
      (`self.Prop_Rotate` (`self.P-38 Right Prop`)))))

(event `EnhancedInput|/Game/P-38/Blueprints/input/IA_Pitch`
  (params (ActionValue :type Boolean) (ElapsedSeconds :type "Float (double-precision)") (TriggeredSeconds :type "Float (double-precision)") (InputAction :type "InputAction Object Reference" :default "/Game/P-38/Blueprints/input/IA_Pitch.IA_Pitch"))
  (:`Triggered`
    (`KismetSystemLibrary.PrintString` (`KismetStringLibrary.Conv_BoolToString` ActionValue))))

(fn `Prop_Rotate`
  (params (Where :type "SceneComponent Object Reference"))
  (`SceneComponent.K2_AddRelativeRotation` Where (`KismetMathLibrary.MakeRotator` (* (`GameplayStatics.GetWorldDeltaSeconds`) (`self.Prop_Rotate Speed`))) false false))

(fn `UserConstructionScript`)